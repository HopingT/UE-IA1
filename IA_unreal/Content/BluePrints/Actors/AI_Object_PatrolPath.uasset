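; AI patrol path actor that aligns a visiting patroller to the direction of its Arrow component.
; OnPatrollerEntered stores the character, opens a Gate and fires the OnPointMet dispatcher.
; While the Gate is open, Tick uses RInterpTo to rotate that character toward the arrow's world rotation.
; OnPatrollerExit closes the Gate, ending the rotation override.
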(event `self.ReceiveTick`
  (params (DeltaSeconds :type "Float (single-precision)"))
  (`/Engine/EditorBlueprintResources/StandardMacros.Gate` true :!label _label
    (:`Exit`
      (`self.K2_SetActorRotation` (`self.Character`) (`KismetMathLibrary.RInterpTo` (`self.K2_GetActorRotation` (`self.Character`)) (`SceneComponent.K2_GetComponentRotation` (`self.Arrow`)) DeltaSeconds) false))))

(event `OnPatrollerEntered`
  (params (character :type "Character Object Reference"))
  (set `self.Character` character)
  (`|ExecutionSequence`
    (:`then_0`
      (goto _label :!via `Open`))
    (:`then_1`
      (`self.OnPointMet`))))

(event `OnPatrollerExit`
  (goto _label :!via `Close`))

(fn `UserConstructionScript`)